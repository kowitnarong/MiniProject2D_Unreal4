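; Checkpoint actor that saves the player's location as a restart point when a Player-tagged actor enters its Box.
; The overlap shows the DoorOpen animation, playing it from the start only if not yet open, then disables looping after a brief delay and marks it open.
; Each such overlap then writes the player character's current location into a fresh MySaveGame, saved to the Restart_Location slot.
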(event `self.Box.OnComponentBeginOverlap`
  (params (OverlappedComponent :type "PrimitiveComponent Object Reference") (OtherActor :type "Actor Object Reference") (OtherComp :type "PrimitiveComponent Object Reference") (OtherBodyIndex :type Integer) (bFromSweep :type Boolean) (SweepResult :type "HitResult Structure (by ref)"))
  (bind _door_open (`self.Door_Open`))
  (if (`self.ActorHasTag` OtherActor "Player")
    (if (not (`self.isOpen`))
      (`PaperFlipbookComponent.PlayFromStart` _door_open))
    (`SceneComponent.SetVisibility` _door_open true false)
    (`KismetSystemLibrary.Delay` 0.2)
    (`PaperFlipbookComponent.SetLooping` (`self.Door_Open`) false)
    (set `self.isOpen` true)
    (bind _returnvalue (`GameplayStatics.CreateSaveGameObject` "/Game/Blueprints/MySaveGame.MySaveGame_C"))
    (bind _output_get (set `self.New_SaveGame` _returnvalue))
    (bind _output_get_2 (set `/Game/Blueprints/MySaveGame.Starting_Location` (`self.K2_GetActorLocation` (`GameplayStatics.GetPlayerCharacter` 0)) _output_get))
    (`GameplayStatics.SaveGameToSlot` (`self.New_SaveGame`) "Restart_Location")))

(fn `UserConstructionScript`)