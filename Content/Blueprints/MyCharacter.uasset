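; Side-scrolling flipbook player character with movement, jumping, a timed melee attack and an HP bar.
; Tick selects the animation, turns the controller to face movement, copies Score to MyGameInstance, and resets score and reloads the level at zero HP.
; Capsule overlaps apply Boom damage with knockback or consume healing items.
; Death, also triggered by P, teleports to the Restart_Location save and costs one HP.
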(event `self.ReceiveBeginPlay`
  (`|ExecutionSequence`
    (:`then_0`
      (bind _asmy_game_instance (cast `/Game/Blueprints/MyGameInstance` (`GameplayStatics.GetGameInstance`)))
      (set `self.Score` (`/Game/Blueprints/MyGameInstance.Score` _asmy_game_instance)))
    (:`then_1`
      (`ActorComponent.SetIsReplicated` (`self.Sprite`) true)
      (bind _returnvalue (`|CreateWidget` "/Game/Blueprints/HP_Bar.HP_Bar_C" (`GameplayStatics.GetPlayerController` 0)))
      (`UserWidget.AddToViewport` _returnvalue 0))))

(event `UpdateAnimation`
  (bind _sprite (`self.Sprite`))
  (if (`self.isDead`)
    (`self.Die`)
    (elif (`self.isAttacking`)
      (`PaperFlipbookComponent.SetFlipbook` _sprite "/Game/Flipbooks/Player/Player_Atk.Player_Atk")
      (elif (`self.onHit`)
        (`PaperFlipbookComponent.SetFlipbook` (`self.Sprite`) "/Game/Flipbooks/Player/Player_Hit.Player_Hit")
        (`|ExecutionSequence`
          (:`then_0`
            (`KismetSystemLibrary.Delay` 0.2)
            (set `self.onHit` false)
            (goto _label :!via `Reset`))
          (:`then_1`
            (`/Engine/EditorBlueprintResources/StandardMacros.DoOnce` false :!label _label
              (:`Completed`
                (`GameplayStatics.PlaySound2D` "/Game/Audio/mixkit-small-hit-in-a-game-2072.mixkit-small-hit-in-a-game-2072" 1.0 1.0 0.0 null null)))))
        (elif (`self.isJumping`)
          (`PaperFlipbookComponent.SetFlipbook` _sprite "/Game/Flipbooks/Player/Player_jump.Player_jump")
          (else
            ;[1 1 1] Handle Animation
            (`PaperFlipbookComponent.SetFlipbook` _sprite (select `bool` (> (`KismetMathLibrary.VSize` (`self.GetVelocity`)) 0.0) :`false` "/Game/Flipbooks/Player/Player_Idle.Player_Idle" :`true` "/Game/Flipbooks/Player/Player_Run.Player_Run" :!type "PaperFlipbook Object Reference"))))))))

(event `InputAxis|MoveRight`
  (params (AxisValue :type "Float (single-precision)"))
  ;[1 1 1] Handle movement
  (if (not (`self.isAttacking`))
    (if (> AxisValue 0.0)
      (set `self.bisMovingRight` true)
      (elif (< AxisValue 0.0)
        (set `self.bisMovingRight` false)))
    (`self.AddMovementInput` (1.0 0.0 0.0) AxisValue)))

(event `self.ReceiveTick`
  (params (DeltaSeconds :type "Float (single-precision)"))
  (bind _returnvalue (`self.GetController`))
  (bind _returnvalue_2 (`self.GetController`))
  ;[1 1 1] Tick - Updates animation
  (`|ExecutionSequence`
    (:`then_0`
      (set `self.HP` (`KismetMathLibrary.FClamp` (`self.HP`) 0.0 3.0))
      (bind _asmy_game_instance (cast `/Game/Blueprints/MyGameInstance` (`GameplayStatics.GetGameInstance`)))
      (set `/Game/Blueprints/MyGameInstance.Score` (`self.Score`) _asmy_game_instance))
    (:`then_1`
      (`self.UpdateAnimation`)
      (`/Engine/EditorBlueprintResources/StandardMacros.CompareFloat` (.x (`MovementComponent.Velocity` (`self.GetMovementComponent`)))
        (:`>`
          (`/Engine/EditorBlueprintResources/StandardMacros.IsValid` _returnvalue_2 :!label _label_2
            (:`Is Valid`
              (`Controller.SetControlRotation` _returnvalue_2 (`KismetMathLibrary.MakeRotator` 0.0)))))
        (:`==`
          (if (`self.bisMovingRight`)
            (goto _label_2)
            (else
              (`/Engine/EditorBlueprintResources/StandardMacros.IsValid` _returnvalue :!label _label_3
                (:`Is Valid`
                  (`Controller.SetControlRotation` _returnvalue (`KismetMathLibrary.MakeRotator` 0.0 0.0 180.0)))))))
        (:`<`
          (goto _label_3))))
    (:`then_2`
      (if (<= (`self.HP`) 0.0)
        (bind _returnvalue_3 (`GameplayStatics.GetCurrentLevelName` true))
        (bind _asmy_game_instance_2 (cast `/Game/Blueprints/MyGameInstance` (`GameplayStatics.GetGameInstance`)))
        (set `/Game/Blueprints/MyGameInstance.Score` 0 _asmy_game_instance_2)
        (`GameplayStatics.OpenLevel` (`KismetStringLibrary.Conv_StringToName` _returnvalue_3))))))

(event `InputAction|Jump`
  (params (Key :type "Key Structure"))
  ;[1 1 1] Handle Jump
  (:`Pressed`
    (`self.Jump` :!label _label_4)
    (set `self.isJumping` true))
  (:`Released`
    (`self.StopJumping` :!label _label_5)))

(event `InputTouch`
  (params (Location :type "Vector Structure") (FingerIndex :type "ETouchIndex Enum"))
  ;[1 1 1] Handle Jump
  (:`Pressed`
    (goto _label_4))
  (:`Released`
    (goto _label_5)))

(event `self.OnLanded`
  (params (Hit :type "HitResult Structure (by ref)"))
  (set `self.isJumping` false))

(event `Die`
  (bind _returnvalue (`GameplayStatics.LoadGameFromSlot` "Restart_Location" :!label _label_6))
  (bind _asmy_save_game (cast `/Game/Blueprints/MySaveGame` _returnvalue))
  (`self.K2_SetActorLocation` (`/Game/Blueprints/MySaveGame.Starting_Location` _asmy_save_game))
  (set `self.isDead` false)
  (set `self.HP` (- (`self.HP`) 1.0)))

(event `Key|F`
  (params (Key :type "Key Structure"))
  (:`Pressed`
    (`/Engine/EditorBlueprintResources/StandardMacros.DoOnce` false :!label _label_7
      (:`Completed`
        (set `self.isAttacking` true)
        (`GameplayStatics.SpawnSound2D` "/Game/Audio/Wav_Attack.Wav_Attack" 1.0 1.0 0.0 null)
        (`|SpawnActorFromClass` "/Game/Blueprints/Melee.Melee_C" (`SceneComponent.K2_GetComponentToWorld` (`self.Arrow_Bullet`)) "Undefined" "OverrideRootScale" null null)
        (`KismetSystemLibrary.Delay` 0.2)
        (set `self.isAttacking` false)
        (`KismetSystemLibrary.Delay` 0.3)
        (goto _label_7 :!via `Reset`)))))

(event `Key|P`
  (params (Key :type "Key Structure"))
  (:`Pressed`
    (goto _label_6)))

(event `Key|LeftMouseButton`
  (params (Key :type "Key Structure"))
  (:`Pressed`
    (goto _label_7)))

(event `self.CapsuleComponent.OnComponentBeginOverlap`
  (params (OverlappedComponent :type "PrimitiveComponent Object Reference") (OtherActor :type "Actor Object Reference") (OtherComp :type "PrimitiveComponent Object Reference") (OtherBodyIndex :type Integer) (bFromSweep :type Boolean) (SweepResult :type "HitResult Structure (by ref)"))
  (bind _returnvalue_x (`KismetMathLibrary.BreakVector` (`self.GetActorForwardVector`)))
  (`|ExecutionSequence`
    (:`then_0`
      (cast `/Game/Blueprints/Enemy/Boom` OtherActor)
      (`KismetSystemLibrary.Delay` 0.1)
      (set `self.HP` (- (`self.HP`) 1.0))
      (set `self.onHit` true)
      (`self.LaunchCharacter` (`KismetMathLibrary.MakeVector` (* _returnvalue_x -750.0) 0.0 400.0) true true))
    (:`then_1`
      (bind _asitem_hp_bp (cast `/Game/Blueprints/item_HP_BP` OtherActor))
      (if (< (`self.HP`) 3.0)
        (set `self.HP` (`KismetMathLibrary.FClamp` (+ (`self.HP`) 1.0) 0.0 3.0))
        (`|ExecutionSequence`
          (:`then_0`
            (`self.K2_DestroyActor` _asitem_hp_bp))
          (:`then_1`
            (`/Engine/EditorBlueprintResources/StandardMacros.DoOnce` false :!label _label_8
              (:`Completed`
                (`GameplayStatics.PlaySound2D` "/Game/Audio/mixkit-game-ball-tap-2073.mixkit-game-ball-tap-2073" 1.0 1.0 0.0 null null)
                (goto _label_8 :!via `Reset`)))))))))

(fn `UserConstructionScript`)