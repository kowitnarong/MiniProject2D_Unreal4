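; DamageUpDown_BP is a hazard that bobs up and down and kills the player character on touch.
; A Delay on Tick drives a FlipFlop that alternately plays and reverses the Animate_Spine timeline, lerping the render component up to 70 units above its starting position.
; That start is cached at BeginPlay as a world location but applied as a relative location.
; Overlapping the Box sets IsDead on MyCharacter.
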(event `self.ReceiveTick`
  (params (DeltaSeconds :type "Float (single-precision)"))
  (bind (_temp_x _temp_y _temp_z) (`KismetMathLibrary.BreakVector` (`self.Temp`)))
  (`KismetSystemLibrary.Delay` (`self.Duration`))
  (`/Engine/EditorBlueprintResources/StandardMacros.FlipFlop`
    (:`A`
      (bind (_direction _speed) (`Timeline|Animate_Spine` :!label _label)
        (:`Update`
          (`SceneComponent.K2_SetRelativeLocation` (`self.RenderComponent`) (`KismetMathLibrary.VLerp` (`KismetMathLibrary.MakeVector` _temp_x _temp_y _temp_z) (`KismetMathLibrary.MakeVector` _temp_x _temp_y (+ _temp_z 70.0)) _speed) false false))))
    (:`B`
      (goto _label :!via `Reverse`))))

(event `self.ReceiveBeginPlay`
  (set `self.Temp` (`SceneComponent.K2_GetComponentLocation` (`self.RenderComponent`))))

(event `self.Box.OnComponentBeginOverlap`
  (params (OverlappedComponent :type "PrimitiveComponent Object Reference") (OtherActor :type "Actor Object Reference") (OtherComp :type "PrimitiveComponent Object Reference") (OtherBodyIndex :type Integer) (bFromSweep :type Boolean) (SweepResult :type "HitResult Structure (by ref)"))
  (bind _asmy_character (cast `/Game/Blueprints/MyCharacter` OtherActor))
  (set `/Game/Blueprints/MyCharacter.isDead` true _asmy_character)
  (`KismetSystemLibrary.Delay` 2.0))

(fn `UserConstructionScript`)