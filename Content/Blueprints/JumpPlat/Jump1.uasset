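; Jump1 is a jump-through platform Blueprint that toggles whether its sprite blocks pawns.
; The sprite ignores the Pawn channel at BeginPlay and blocks it after the player character begins overlapping the Box.
; The delay before blocking is shorter when the player's capsule center is above the sprite, longer otherwise.
; Leaving the Box returns the sprite to ignoring pawns.
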(event `self.ReceiveBeginPlay`
  (`PrimitiveComponent.SetCollisionResponseToChannel` (`self.Decorations__32x32__Sprite_15`) "ECC_Pawn" "ECR_Ignore"))

(event `self.Box.OnComponentBeginOverlap`
  (params (OverlappedComponent :type "PrimitiveComponent Object Reference") (OtherActor :type "Actor Object Reference") (OtherComp :type "PrimitiveComponent Object Reference") (OtherBodyIndex :type Integer) (bFromSweep :type Boolean) (SweepResult :type "HitResult Structure (by ref)"))
  (bind _returnvalue (`GameplayStatics.GetPlayerCharacter` 0))
  (if (== OtherActor _returnvalue)
    (if (> (.z (`SceneComponent.K2_GetComponentLocation` (`Character.CapsuleComponent` _returnvalue))) (.z (`SceneComponent.K2_GetComponentLocation` (`self.Decorations__32x32__Sprite_15`))))
      (`KismetSystemLibrary.Delay` 0.05)
      (else
        (`KismetSystemLibrary.Delay` 0.1)))
    (`PrimitiveComponent.SetCollisionResponseToChannel` (`self.Decorations__32x32__Sprite_15`) "ECC_Pawn" "ECR_Block")))

(event `self.Box.OnComponentEndOverlap`
  (params (OverlappedComponent :type "PrimitiveComponent Object Reference") (OtherActor :type "Actor Object Reference") (OtherComp :type "PrimitiveComponent Object Reference") (OtherBodyIndex :type Integer))
  (if (== OtherActor (`GameplayStatics.GetPlayerCharacter` 0))
    (`PrimitiveComponent.SetCollisionResponseToChannel` (`self.Decorations__32x32__Sprite_15`) "ECC_Pawn" "ECR_Ignore")))

(fn `UserConstructionScript`)