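; Jump platform that tilts around its pitch axis toward whichever side the player character stands on.
; BoxL and BoxR overlaps set per-side flags, clearing the check flag half a second after exit.
; Tick uses those flags to drive RotatingMovement at a near-constant rate in opposite directions.
; Once released, delayed steps ease the rate back through reversal until pitch crosses zero, then rotation stops and snaps level.
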(event `self.BoxL.OnComponentBeginOverlap`
  (params (OverlappedComponent :type "PrimitiveComponent Object Reference") (OtherActor :type "Actor Object Reference") (OtherComp :type "PrimitiveComponent Object Reference") (OtherBodyIndex :type Integer) (bFromSweep :type Boolean) (SweepResult :type "HitResult Structure (by ref)"))
  (cast `/Game/Blueprints/MyCharacter` OtherActor)
  (set `self.CheckLeft` true)
  (set `self.isMovingLeft` true)
  (set `self.isMovingRight` false))

(event `self.ReceiveTick`
  (params (DeltaSeconds :type "Float (single-precision)"))
  (bind _rotatingmovement (`self.RotatingMovement`))
  (bind _rotatingmovement_2 (`self.RotatingMovement`))
  (bind (_returnvalue_roll _returnvalue_pitch) (`KismetMathLibrary.BreakRotator` (`SceneComponent.K2_GetComponentRotation` (`self.RenderComponent`))))
  (bind (_returnvalue_roll_2 _returnvalue_pitch_2) (`KismetMathLibrary.BreakRotator` (`SceneComponent.K2_GetComponentRotation` (`self.RenderComponent`))))
  (bind (_rotationrate_roll _rotationrate_pitch) (`KismetMathLibrary.BreakRotator` (`RotatingMovementComponent.RotationRate` (`self.RotatingMovement`))))
  (bind (_rotationrate_roll_2 _rotationrate_pitch_2) (`KismetMathLibrary.BreakRotator` (`RotatingMovementComponent.RotationRate` (`self.RotatingMovement`))))
  (`|ExecutionSequence`
    (:`then_0`
      (if (`self.isMovingRight`)
        _
        (elif (`self.CheckLeft`)
          (set `RotatingMovementComponent.RotationRate` (`KismetMathLibrary.MakeRotator` 0.0 (+ DeltaSeconds 35.0)) _rotatingmovement_2)
          (elif (> _returnvalue_pitch_2 0.0)
            (`KismetSystemLibrary.Delay` 0.2)
            (set `RotatingMovementComponent.RotationRate` (`KismetMathLibrary.MakeRotator` 0.0 (- _rotationrate_pitch_2 1.0)) _rotatingmovement_2)
            (else
              (set `RotatingMovementComponent.RotationRate` (struct) _rotatingmovement_2)
              (set `self.isMovingLeft` false)
              (`SceneComponent.K2_SetWorldRotation` :`self` (`self.RenderComponent`)))))))
    (:`then_1`
      (if (`self.isMovingLeft`)
        _
        (elif (`self.CheckRight`)
          (set `RotatingMovementComponent.RotationRate` (`KismetMathLibrary.MakeRotator` 0.0 (- DeltaSeconds 35.0)) _rotatingmovement)
          (elif (< _returnvalue_pitch 0.0)
            (`KismetSystemLibrary.Delay` 0.2)
            (set `RotatingMovementComponent.RotationRate` (`KismetMathLibrary.MakeRotator` 0.0 (+ _rotationrate_pitch 1.0)) _rotatingmovement)
            (else
              (set `RotatingMovementComponent.RotationRate` (struct) _rotatingmovement)
              (set `self.isMovingRight` false)
              (`SceneComponent.K2_SetWorldRotation` :`self` (`self.RenderComponent`)))))))))

(event `self.BoxL.OnComponentEndOverlap`
  (params (OverlappedComponent :type "PrimitiveComponent Object Reference") (OtherActor :type "Actor Object Reference") (OtherComp :type "PrimitiveComponent Object Reference") (OtherBodyIndex :type Integer))
  (cast `/Game/Blueprints/MyCharacter` OtherActor)
  (`KismetSystemLibrary.Delay` 0.5)
  (set `self.CheckLeft` false))

(event `self.BoxR.OnComponentBeginOverlap`
  (params (OverlappedComponent :type "PrimitiveComponent Object Reference") (OtherActor :type "Actor Object Reference") (OtherComp :type "PrimitiveComponent Object Reference") (OtherBodyIndex :type Integer) (bFromSweep :type Boolean) (SweepResult :type "HitResult Structure (by ref)"))
  (cast `/Game/Blueprints/MyCharacter` OtherActor)
  (set `self.CheckRight` true)
  (set `self.isMovingRight` true)
  (set `self.isMovingLeft` false))

(event `self.BoxR.OnComponentEndOverlap`
  (params (OverlappedComponent :type "PrimitiveComponent Object Reference") (OtherActor :type "Actor Object Reference") (OtherComp :type "PrimitiveComponent Object Reference") (OtherBodyIndex :type Integer))
  (cast `/Game/Blueprints/MyCharacter` OtherActor)
  (`KismetSystemLibrary.Delay` 0.5)
  (set `self.CheckRight` false))

(fn `UserConstructionScript`)