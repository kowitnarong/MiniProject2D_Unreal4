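; Level-transition door that sends the player to the level named in LevelName when they touch its Box trigger.
; An overlap by an actor tagged Player plays DoorOpen from the start unless IsOpen is set, then makes it visible.
; Short delays turn off the animation's looping and then open the level.
; IsOpen is only read here, never set.
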(event `self.Box.OnComponentBeginOverlap`
  (params (OverlappedComponent :type "PrimitiveComponent Object Reference") (OtherActor :type "Actor Object Reference") (OtherComp :type "PrimitiveComponent Object Reference") (OtherBodyIndex :type Integer) (bFromSweep :type Boolean) (SweepResult :type "HitResult Structure (by ref)"))
  (bind _door_open (`self.Door_Open`))
  (if (`self.ActorHasTag` OtherActor "Player")
    (if (not (`self.isOpen`))
      (`PaperFlipbookComponent.PlayFromStart` _door_open))
    (`SceneComponent.SetVisibility` _door_open true false)
    (`KismetSystemLibrary.Delay` 0.2)
    (`PaperFlipbookComponent.SetLooping` (`self.Door_Open`) false)
    (`KismetSystemLibrary.Delay` 0.4)
    (`GameplayStatics.OpenLevel` (`self.Level Name`))))

(fn `UserConstructionScript`)